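; BP_Test is a test actor that acts as a temporarily disappearing platform, dropping collision after a Pawn lands on it while staying visible.
; StaticMesh hit events are filtered to Pawns with a straight-down impact normal, indicating contact from above.
; Chained event timers disable collision after a short delay, then restore query and physics collision, with debug prints along the way.
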(event `self.ReceiveBeginPlay`
  (add `PrimitiveComponent.OnComponentHit` (`self.StaticMesh`) (delegate `CustomEvent`)))

(event `CustomEvent`
  (params (HitComponent :type "PrimitiveComponent Object Reference") (OtherActor :type "Actor Object Reference") (OtherComp :type "PrimitiveComponent Object Reference") (NormalImpulse :type "Vector Structure") (Hit :type "HitResult Structure (by ref)"))
  (if (and (`GameplayStatics.ObjectIsA` OtherActor "/Script/Engine.Pawn") (`KismetMathLibrary.NearlyEqual_FloatFloat` (.z (`.ImpactNormal` (`GameplayStatics.BreakHitResult` Hit))) -1.0))
    (`KismetSystemLibrary.K2_SetTimerDelegate` (delegate `CustomEvent_0`) 1.0)
    (`KismetSystemLibrary.PrintString` "Disable collision")))

(event `CustomEvent_0`
  (`PrimitiveComponent.SetCollisionEnabled` (`self.StaticMesh`) "NoCollision")
  (`KismetSystemLibrary.K2_SetTimerDelegate` (delegate `CustomEvent_1`) 2.0))

(event `CustomEvent_1`
  (`PrimitiveComponent.SetCollisionEnabled` (`self.StaticMesh`) "QueryAndPhysics")
  (`KismetSystemLibrary.PrintString` "Enable collision"))

(fn `UserConstructionScript`)