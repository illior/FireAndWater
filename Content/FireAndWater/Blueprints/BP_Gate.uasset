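; BP_Gate is a gate that slides its Gate component vertically between open and closed Z positions.
; Open and Close each restart a shared per-frame looping timer that moves the gate until it nears its target, then snaps and stops.
; Opening uses constant-speed interpolation, while closing uses eased FInterpTo, with debug prints at timer start and stop.
; Timeline-based OpenGraph and CloseGraph alternatives exist but are never run.
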(event `Open`
  (`KismetSystemLibrary.K2_ClearAndInvalidateTimerHandle` (`self.InterpolateTimer`))
  (bind _returnvalue (`KismetSystemLibrary.K2_SetTimerDelegate` (delegate `OpenInterpolate`) (`GameplayStatics.GetWorldDeltaSeconds`) true true))
  (set `self.InterpolateTimer` _returnvalue)
  (`KismetSystemLibrary.PrintString` "Start Open Timer"))

(event `OpenInterpolate`
  (bind (_relativelocation_x _relativelocation_y _relativelocation_z) (`KismetMathLibrary.BreakVector` (`SceneComponent.RelativeLocation` (`self.Gate`))))
  (bind (_relativelocation_x_2 _relativelocation_y_2) (`KismetMathLibrary.BreakVector` (`SceneComponent.RelativeLocation` (`self.Gate`))))
  (bind (_relativelocation_x_3 _relativelocation_y_3) (`KismetMathLibrary.BreakVector` (`SceneComponent.RelativeLocation` (`self.Gate`))))
  (bind _returnvalue (`KismetMathLibrary.FInterpTo_Constant` _relativelocation_z (`self.OpenPositionZ`) (`GameplayStatics.GetWorldDeltaSeconds`) 150.0))
  (if (`KismetMathLibrary.NearlyEqual_FloatFloat` _returnvalue (`self.OpenPositionZ`) 0.1)
    (`SceneComponent.K2_SetRelativeLocation` (`self.Gate`) (`KismetMathLibrary.MakeVector` _relativelocation_x_2 _relativelocation_y_2 (`self.OpenPositionZ`)) false false)
    (`KismetSystemLibrary.K2_ClearAndInvalidateTimerHandle` (`self.InterpolateTimer`))
    (`KismetSystemLibrary.PrintString` "Stop Open Timer")
    (else
      (`SceneComponent.K2_SetRelativeLocation` (`self.Gate`) (`KismetMathLibrary.MakeVector` _relativelocation_x_3 _relativelocation_y_3 _returnvalue) false false))))

(event `Close`
  (`KismetSystemLibrary.K2_ClearAndInvalidateTimerHandle` (`self.InterpolateTimer`))
  (bind _returnvalue (`KismetSystemLibrary.K2_SetTimerDelegate` (delegate `CloseInterpolate`) (`GameplayStatics.GetWorldDeltaSeconds`) true true))
  (set `self.InterpolateTimer` _returnvalue)
  (`KismetSystemLibrary.PrintString` "Start Close Timer"))

(event `CloseInterpolate`
  (bind (_relativelocation_x _relativelocation_y) (`KismetMathLibrary.BreakVector` (`SceneComponent.RelativeLocation` (`self.Gate`))))
  (bind (_relativelocation_x_2 _relativelocation_y_2) (`KismetMathLibrary.BreakVector` (`SceneComponent.RelativeLocation` (`self.Gate`))))
  (bind (_relativelocation_x_3 _relativelocation_y_3 _relativelocation_z) (`KismetMathLibrary.BreakVector` (`SceneComponent.RelativeLocation` (`self.Gate`))))
  (bind _returnvalue (`KismetMathLibrary.FInterpTo` _relativelocation_z (`self.ClosePositionZ`) (`GameplayStatics.GetWorldDeltaSeconds`) 4.0))
  (if (`KismetMathLibrary.NearlyEqual_FloatFloat` _returnvalue (`self.ClosePositionZ`) 1.0)
    (`SceneComponent.K2_SetRelativeLocation` (`self.Gate`) (`KismetMathLibrary.MakeVector` _relativelocation_x _relativelocation_y (`self.ClosePositionZ`)) false false)
    (`KismetSystemLibrary.K2_ClearAndInvalidateTimerHandle` (`self.InterpolateTimer`))
    (`KismetSystemLibrary.PrintString` "Stop Close Timer")
    (else
      (`SceneComponent.K2_SetRelativeLocation` (`self.Gate`) (`KismetMathLibrary.MakeVector` _relativelocation_x_2 _relativelocation_y_2 _returnvalue) false false))))

(fn `UserConstructionScript`)