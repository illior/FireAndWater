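; BP_DirectionWind is a cave wind volume that, while Active, carries FAW characters along its Direction.
; On overlap it resets jumps, launches the character along Direction with damped horizontal momentum, and tracks it.
; Tick keeps tracked characters in Flying mode, updates their velocity through CalcVelocity, and draws a debug arrow.
; Leaving the active volume untracks the character and switches it to Falling.
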(event `self.ReceiveActorBeginOverlap`
  (params (OtherActor :type "Actor Object Reference"))
  (if (`self.Active`)
    (bind _asfawbase_character (cast `FAWBaseCharacter` OtherActor))
    (`FAWBaseCharacter.ResetJumps` _asfawbase_character)
    (`KismetArrayLibrary.Array_Add` (`self.Characters`) _asfawbase_character)
    (bind _charactermovement (`Character.CharacterMovement` _asfawbase_character))
    (set `MovementComponent.Velocity` (+ (* (`self.Direction`) 750.0) (`KismetMathLibrary.MakeVector` (.x (/ (`MovementComponent.Velocity` _charactermovement) 4.0)) (.y (/ (`MovementComponent.Velocity` _charactermovement) 4.0)))) _charactermovement)))

(event `self.ReceiveActorEndOverlap`
  (params (OtherActor :type "Actor Object Reference"))
  (if (`self.Active`)
    (bind _asfawbase_character (cast `FAWBaseCharacter` OtherActor))
    (`KismetArrayLibrary.Array_RemoveItem` (`self.Characters`) _asfawbase_character)
    (`CharacterMovementComponent.SetMovementMode` (`Character.CharacterMovement` _asfawbase_character) "MOVE_Falling" 0)))

(event `self.ReceiveTick`
  (params (DeltaSeconds :type "Float (single-precision)"))
  (bind _returnvalue (`SceneComponent.K2_GetComponentLocation` (`self.Box`)))
  (if (`self.Active`)
    (`KismetSystemLibrary.DrawDebugArrow` _returnvalue (+ _returnvalue (* (`self.Direction`) 200.0)) 200.0 (struct :`R` 1.0 :`A` 1.0) 0.0 3.0)
    (for _array_element (`self.Characters`)
      (if (not (`|EnumEquality` (`CharacterMovementComponent.MovementMode` (`Character.CharacterMovement` _array_element)) "MOVE_Flying"))
        (`CharacterMovementComponent.SetMovementMode` (`Character.CharacterMovement` _array_element) "MOVE_Flying" 0))
      (bind _charactermovement (`Character.CharacterMovement` _array_element))
      (bind (_returnvalue_x _returnvalue_y _returnvalue_z) (`KismetMathLibrary.BreakVector` (+ (`MovementComponent.Velocity` _charactermovement) (* (`self.Direction`) (* (`self.Multiply`) (`GameplayStatics.GetWorldDeltaSeconds`))))))
      (set `MovementComponent.Velocity` (`KismetMathLibrary.MakeVector` _returnvalue_x _returnvalue_y (`KismetMathLibrary.FClamp` _returnvalue_z -1500.0 500.0)) _charactermovement))))

(fn `UserConstructionScript`)