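; BP_CaveGate is a cave gate with two doors that swing open when its Open event is called.
; Open starts a fast looping timer that runs OpenUpdate, advancing the right door's yaw by world delta time at a fixed rate.
; The left door derives its rotation from the right door's with negated yaw, and the timer clears once the swing passes a right angle.
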(event `Open`
  (bind _returnvalue (`KismetSystemLibrary.K2_SetTimerDelegate` (delegate `OpenUpdate`) 0.005 true true))
  (set `self.TimerHandle` _returnvalue))

(event `OpenUpdate`
  (bind _rightdoor (`self.RightDoor`))
  (bind (_relativerotation_roll _relativerotation_pitch _relativerotation_yaw) (`KismetMathLibrary.BreakRotator` (`SceneComponent.RelativeRotation` _rightdoor)))
  (bind _returnvalue (+ _relativerotation_yaw (* (/ 90.0 1.5) (`GameplayStatics.GetWorldDeltaSeconds`))))
  (`SceneComponent.K2_SetRelativeRotation` _rightdoor (`KismetMathLibrary.MakeRotator` _relativerotation_roll _relativerotation_pitch _returnvalue) false false)
  (`SceneComponent.K2_SetRelativeRotation` (`self.LeftDoor`) (`KismetMathLibrary.MakeRotator` _relativerotation_roll _relativerotation_pitch (* _returnvalue -1.0)) false false)
  (if (> _returnvalue 90.0)
    (`KismetSystemLibrary.K2_ClearAndInvalidateTimerHandle` (`self.TimerHandle`))))

(fn `UserConstructionScript`)