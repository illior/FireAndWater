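; BP_CableWay is a cableway in the cave area that carries a Room component along a spline.
; The construction script adds a black cable component at each spline point, aimed at the next point, with its length shortened below the segment's spline distance.
; While Active, Tick moves the Room by distance along the spline at Speed, snapping back to the start after passing the end.
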(event `self.ReceiveTick`
  (params (DeltaSeconds :type "Float (single-precision)"))
  (if (`self.bActive`)
    (`SceneComponent.K2_SetRelativeLocation` (`self.Room`) (`SplineComponent.GetLocationAtDistanceAlongSpline` (`self.Spline`) (`self.CurrentDistance`) "Local") false false)
    (bind _output_get (set `self.CurrentDistance` (+ (`self.CurrentDistance`) (* (`self.Speed`) DeltaSeconds))))
    (if (> _output_get (`SplineComponent.GetSplineLength` (`self.Spline`)))
      (set `self.CurrentDistance` 0.0))))

(fn `UserConstructionScript`
  (bind _spline (`self.Spline`))
  (for _index (range (`SplineComponent.GetNumberOfSplinePoints` (`self.Spline`)))
    (bind _returnvalue (`AddComponent|NODE_AddCableComponent-0` :`RelativeTransform` (`SplineComponent.GetTransformAtSplinePoint` (`self.Spline`) _index "Local" false)))
    (bind _returnvalue_2 (+ _index 1))
    (set `CableComponent.EndLocation` (`SplineComponent.GetLocationAtSplinePoint` (`self.Spline`) _returnvalue_2 "Local") _returnvalue)
    (set `CableComponent.CableLength` (/ (- (`SplineComponent.GetDistanceAlongSplineAtSplinePoint` _spline _returnvalue_2) (`SplineComponent.GetDistanceAlongSplineAtSplinePoint` _spline _index)) 1.5) _returnvalue)
    (`PrimitiveComponent.SetMaterial` _returnvalue 0 "/Game/FireAndWater/Materials/MI_Black.MI_Black")))