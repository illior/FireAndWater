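; Trap platform for the cave level that throws a Fire and Water character forward into a jump and flips when landed on.
; A downward hit normal on an active platform disables it, launches the character and starts a fast looping timer.
; The timer linearly rotates the root's pitch between two angles.
; After TimeToComplete it re-arms, clears the timer and swaps the angles, so the next trigger rotates back.
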(event `self.ReceiveHit`
  (params (MyComp :type "PrimitiveComponent Object Reference") (Other :type "Actor Object Reference") (OtherComp :type "PrimitiveComponent Object Reference") (bSelfMoved :type Boolean) (HitLocation :type "Vector Structure") (HitNormal :type "Vector Structure") (NormalImpulse :type "Vector Structure") (Hit :type "HitResult Structure (by ref)"))
  (bind _asfawbase_character (cast `FAWBaseCharacter` Other))
  (if (and (< (.z HitNormal) -0.1) (`self.bPlatformActive`))
    (set `self.bPlatformActive` false)
    (`self.LaunchCharacter` _asfawbase_character)
    (set `self.CurrentTime` 0.0)
    (bind _returnvalue (`KismetSystemLibrary.K2_SetTimerDelegate` (`|CreateDelegate` :!event `MovePlatform`) 0.005 true true))
    (set `self.TimerHandle` _returnvalue)))

(event `MovePlatform`
  (set `self.CurrentTime` (+ (`self.CurrentTime`) (* (`GameplayStatics.GetWorldDeltaSeconds`) 2.0)))
  (`SceneComponent.K2_SetRelativeRotation` (`self.PlatformRoot`) (`KismetMathLibrary.MakeRotator` 0.0 (`|EaseFunction` "Linear" (`self.CurrentTime`) (`self.InitialAngle`) (`self.TargetAngle`))) false false)
  (if (>= (`self.CurrentTime`) (`self.TimeToComplete`))
    (set `self.bPlatformActive` true)
    (`KismetSystemLibrary.K2_ClearAndInvalidateTimerHandle` (`self.TimerHandle`))
    (`self.Swap`)))

(fn `LaunchCharacter`
  (params (Character :type "FAWBaseCharacter Object Reference"))
  (set `MovementComponent.Velocity` (* (`self.GetActorForwardVector` Character) 300.0) (`Pawn.GetMovementComponent` Character))
  (`Character.Jump` Character))

(fn `Swap`
  (locals (Temp :type "Float (double-precision)" :default 0.0))
  (set `local.Temp` (`self.TargetAngle`))
  (set `self.TargetAngle` (`self.InitialAngle`))
  (set `self.InitialAngle` (`local.Temp`)))

(fn `UserConstructionScript`)