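; Carryable cave crystal that a character picks up with a hold interaction, limited to one crystal per character.
; On hold completion it checks the activator's attached actors for another crystal, then either snaps to the BackPack socket without collision or re-enables itself after a short delay.
; When the carrier dies, it detaches, moves to a random point around that player's last checkpoint and becomes collidable and interactable again.
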(event `self.ReceiveBeginPlay`
  (add `self.OnCompleteHold` (delegate `OnCompleteHold_Event`)))

(event `OnCompleteHold_Event` :!signature `self.OnCompleteHold`
  (params (ActivatedActor :type "FAWInteractableActor Object Reference") (ActivatedBy :type "Pawn Object Reference"))
  (set `self.CanTake` true)
  (for _array_element (`self.GetAttachedActors` ActivatedBy true false)
    (if (`GameplayStatics.ObjectIsA` _array_element "BP_CaveCrystal_C")
      (set `self.CanTake` false)
      (break)))
  (if (`self.CanTake`)
    (bind _ascharacter (cast `Character` ActivatedBy))
    (`self.TakeCrystal` (`Character.Mesh` _ascharacter))
    (else
      (`KismetSystemLibrary.Delay` 1.0)
      (`self.Multicast_SetEnabled` true))))

(event `TakeCrystal`
  (params (NewOwner :type "SceneComponent Object Reference"))
  (`self.K2_AttachToComponent` NewOwner "BackPack" "SnapToTarget" "SnapToTarget" "SnapToTarget")
  (`PrimitiveComponent.SetCollisionEnabled` (`self.StaticMesh`) "NoCollision")
  (bind _asfawbase_character (cast `FAWBaseCharacter` (`ActorComponent.GetOwner` NewOwner)))
  (add `FAWHealthComponent.OnDeath` (`self.GetComponentByClass` _asfawbase_character "/Script/FireAndWater.FAWHealthComponent") (delegate `OnOwnerDeath`)))

(event `OnOwnerDeath`
  (bind _asfawbase_character (cast `FAWBaseCharacter` (`self.GetAttachParentActor`)))
  (bind _asfawplayer_state (cast `FAWPlayerState` (`Pawn.PlayerState` _asfawbase_character)))
  (`self.K2_DetachFromActor` "KeepWorld" "KeepWorld" "KeepWorld")
  (`self.BackToCheckPoint` (`KismetMathLibrary.RandomPointInBoundingBox` (`self.K2_GetActorLocation` (`FAWPlayerState.GetLastCheckPoint` _asfawplayer_state)) (400.0 400.0 0.0)))
  (`self.Multicast_SetEnabled` true))

(event `BackToCheckPoint`
  (params (Location :type "Vector Structure"))
  (`self.K2_SetActorLocationAndRotation` Location)
  (`PrimitiveComponent.SetCollisionEnabled` (`self.StaticMesh`) "QueryAndPhysics"))

(fn `UserConstructionScript`)