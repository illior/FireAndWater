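; BP_MovingStep is a cave step that slides its static mesh along local X between a closed and an open position.
; Show and Hide set the target X and restart a looping timer, which appears to drive Moving.
; Moving shifts the mesh by frame delta at a speed covering the full range in about one second, clamped to both limits, and clears the timer on arrival.
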(event `Hide`
  (if (`KismetSystemLibrary.K2_IsTimerActiveHandle` (`self.TimerHandle`))
    (`KismetSystemLibrary.K2_ClearAndInvalidateTimerHandle` (`self.TimerHandle`)))
  (set `self.TargetX` (`self.CloseX`))
  (bind _returnvalue (`KismetSystemLibrary.K2_SetTimerDelegate` (`|CreateDelegate` :!event `Moving`) 0.005 true true))
  (set `self.TimerHandle` _returnvalue))

(event `Moving`
  (bind _staticmesh (`self.StaticMesh`))
  (bind (_relativelocation_x _relativelocation_y _relativelocation_z) (`KismetMathLibrary.BreakVector` (`SceneComponent.RelativeLocation` _staticmesh)))
  (bind _relativelocation_x_2 (`KismetMathLibrary.BreakVector` (`SceneComponent.RelativeLocation` (`self.StaticMesh`))))
  (bind _returnvalue (`KismetMathLibrary.FClamp` (+ _relativelocation_x (* (* (`KismetMathLibrary.Abs` (- (`self.OpenX`) (`self.CloseX`))) (select `bool` (< _relativelocation_x_2 (`self.TargetX`)) :`false` -1.0 :`true` 1.0)) (`GameplayStatics.GetWorldDeltaSeconds`))) (`self.CloseX`) (`self.OpenX`)))
  (`SceneComponent.K2_SetRelativeLocation` _staticmesh (`KismetMathLibrary.MakeVector` _returnvalue _relativelocation_y _relativelocation_z) false false)
  (if (`KismetMathLibrary.NearlyEqual_FloatFloat` _returnvalue (`self.TargetX`))
    (`KismetSystemLibrary.K2_ClearAndInvalidateTimerHandle` (`self.TimerHandle`))))

(event `Show`
  (if (`KismetSystemLibrary.K2_IsTimerActiveHandle` (`self.TimerHandle`))
    (`KismetSystemLibrary.K2_ClearAndInvalidateTimerHandle` (`self.TimerHandle`)))
  (set `self.TargetX` (`self.OpenX`))
  (bind _returnvalue (`KismetSystemLibrary.K2_SetTimerDelegate` (`|CreateDelegate` :!event `Moving`) 0.005 true true))
  (set `self.TimerHandle` _returnvalue))

(fn `UserConstructionScript`)