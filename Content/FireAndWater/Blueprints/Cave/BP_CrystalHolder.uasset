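; Cave crystal holder that lets an actor insert or remove a BP_CaveCrystal by completing a hold interaction.
; When active, it passes the attached crystal to the activator's mesh component through TakeCrystal.
; When inactive, it snaps a crystal attached to the activator onto its static mesh and enables the crystal's collision.
; Each transfer updates Activated and broadcasts the state change.
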(event `self.ReceiveBeginPlay`
  (`|ExecutionSequence`
    (:`then_1`
      (add `self.OnCompleteHold` (delegate `OnCompleteHold_Event`)))))

(event `OnCompleteHold_Event` :!signature `self.OnCompleteHold`
  (params (ActivatedActor :type "FAWInteractableActor Object Reference") (ActivatedBy :type "Pawn Object Reference"))
  (if (`self.bActivated`)
    (for _array_element (`self.GetAttachedActors` true)
      (bind _asbp_cave_crystal (cast `/Game/FireAndWater/Blueprints/Cave/BP_CaveCrystal` _array_element))
      (`/Game/FireAndWater/Blueprints/Cave/BP_CaveCrystal.TakeCrystal` _asbp_cave_crystal (`self.GetComponentByClass` ActivatedBy "/Script/Engine.MeshComponent"))
      (bind _output_get (set `self.bActivated` false))
      (`self.OnStateChanged` _output_get)
      (break))
    (else
      (for _array_element_2 (`self.GetAttachedActors` ActivatedBy true false)
        (bind _asbp_cave_crystal_2 (cast `/Game/FireAndWater/Blueprints/Cave/BP_CaveCrystal` _array_element_2))
        (`self.AddCrystal` _asbp_cave_crystal_2)
        (break)))))

(event `AddCrystal`
  (params (InActor :type "/Game/FireAndWater/Blueprints/Cave/BP_CaveCrystal Object Reference"))
  (`self.K2_AttachToComponent` InActor (`self.StaticMesh`) "None" "SnapToTarget" "SnapToTarget" "KeepWorld" true)
  (bind _output_get (set `self.bActivated` true))
  (`self.OnStateChanged` _output_get)
  (`PrimitiveComponent.SetCollisionEnabled` (`/Game/FireAndWater/Blueprints/Cave/BP_CaveCrystal.StaticMesh` InActor) "QueryAndPhysics"))

(fn `UserConstructionScript`)