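; Cave bridge actor that pitches in steps as Hold and Release events arrive, each shifting its target angle by half the open angle.
; While the bridge is open, these events start a looping timer if none is running, apparently driving MoveBridge.
; MoveBridge turns pitch toward the target at a fixed rate and stops the timer when close.
; Settling near zero pitch clears IsOpen, so further Hold and Release calls are ignored.
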(event `Hold`
  (if (`self.bIsOpen`)
    (set `self.TargetAngle` (- (`self.TargetAngle`) (/ (`self.OpenAngle`) 2.0)))
    (if (not (`KismetSystemLibrary.K2_IsTimerActiveHandle` (`self.TimerHandle`)))
      (bind _returnvalue (`KismetSystemLibrary.K2_SetTimerDelegate` (`|CreateDelegate` :!event `MoveBridge`) 0.001 true true))
      (set `self.TimerHandle` _returnvalue))))

(event `Release`
  (if (`self.bIsOpen`)
    (set `self.TargetAngle` (+ (`self.TargetAngle`) (/ (`self.OpenAngle`) 2.0)))
    (if (not (`KismetSystemLibrary.K2_IsTimerActiveHandle` (`self.TimerHandle`)))
      (bind _returnvalue (`KismetSystemLibrary.K2_SetTimerDelegate` (`|CreateDelegate` :!event `MoveBridge`) 0.001 true true))
      (set `self.TimerHandle` _returnvalue))))

(event `MoveBridge`
  (bind (_returnvalue_roll _returnvalue_pitch) (`KismetMathLibrary.BreakRotator` (`self.K2_GetActorRotation`)))
  (bind (_returnvalue_roll_2 _returnvalue_pitch_2 _returnvalue_yaw) (`KismetMathLibrary.BreakRotator` (`self.K2_GetActorRotation`)))
  (bind _returnvalue (+ _returnvalue_pitch_2 (* 20.0 (`KismetMathLibrary.SelectFloat` -1.0 1.0 (> _returnvalue_pitch (`self.TargetAngle`))) (`GameplayStatics.GetWorldDeltaSeconds`))))
  (`self.K2_SetActorRotation` (`KismetMathLibrary.MakeRotator` _returnvalue_roll_2 _returnvalue _returnvalue_yaw))
  (if (`KismetMathLibrary.NearlyEqual_FloatFloat` _returnvalue (`self.TargetAngle`) 0.5)
    (`KismetSystemLibrary.K2_ClearAndInvalidateTimerHandle` (`self.TimerHandle`))
    (if (`KismetMathLibrary.NearlyEqual_FloatFloat` _returnvalue 0.0 0.5)
      (set `self.bIsOpen` false))))

(fn `UserConstructionScript`)