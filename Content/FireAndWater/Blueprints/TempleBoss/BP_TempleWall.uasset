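; BP_TempleWall is a temple boss wall that fires a row of spear ejectors in volleys.
; The construction script spawns BP_SpearEjector child actors along local X from Length, Distance and Scale, storing them in Ejectors.
; ShotFromAll fires them all at once or staggers them with a looping timer, in forward or reverse order.
; Each volley then sets a delayed timer event, and EndShooting calls the OnEndShooting dispatcher.
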(event `EndShooting`
  (`self.OnEndShooting`))

(event `ShotFromAll`
  (params (Type :type "/Game/FireAndWater/Blueprints/TempleBoss/BPE_ShotTypes Enum" :default "NewEnumerator0") (Reverse :type Boolean))
  (set `self.Reverse` Reverse)
  (switch `/Game/FireAndWater/Blueprints/TempleBoss/BPE_ShotTypes` Type
    (:`NewEnumerator0`
      (if (`self.Reverse`)
        (bind (_arrayindex _arrayelement) (`/Engine/EditorBlueprintResources/StandardMacros.ReverseForEachLoop` (`self.Ejectors`))
          (:`LoopBody`
            (`/Game/FireAndWater/Blueprints/TempleBoss/BP_SpearEjector.Shot` _arrayelement))
          (:`Completed`
            (`KismetSystemLibrary.K2_SetTimerDelegate` (`|CreateDelegate` :!event `EndShooting`) 1.0 :!label _label)))
        (else
          (for _array_element (`self.Ejectors`)
            (`/Game/FireAndWater/Blueprints/TempleBoss/BP_SpearEjector.Shot` _array_element))
          (goto _label))))
    (:`NewEnumerator1`
      (`KismetSystemLibrary.K2_ClearAndInvalidateTimerHandle` (`self.TimerHandle`))
      (set `self.Index` (`KismetMathLibrary.SelectInt` (- (`KismetArrayLibrary.Array_Length` (`self.Ejectors`)) 1) 0 (`self.Reverse`)))
      (bind _returnvalue (`KismetSystemLibrary.K2_SetTimerDelegate` (delegate `TimerLoop`) 0.15 true))
      (set `self.TimerHandle` _returnvalue))))

(event `TimerLoop`
  (if (`KismetArrayLibrary.Array_IsValidIndex` (`self.Ejectors`) (`self.Index`))
    (`/Game/FireAndWater/Blueprints/TempleBoss/BP_SpearEjector.Shot` (`|GetArrayItem` (`self.Ejectors`) (`self.Index`)))
    (set `self.Index` (+ (`self.Index`) (`KismetMathLibrary.SelectInt` -1 1 (`self.Reverse`))))
    (else
      (`KismetSystemLibrary.K2_ClearAndInvalidateTimerHandle` (`self.TimerHandle`))
      (`KismetSystemLibrary.K2_SetTimerDelegate` (`|CreateDelegate` :!event `EndShooting`) 1.0))))

(fn `UserConstructionScript`
  (`KismetArrayLibrary.Array_Clear` (`self.Ejectors`))
  (for _index (range (+ (`self.Length`) 1))
    (bind _returnvalue (`AddComponent|NODE_AddChildActorComponent-0` :`RelativeTransform` (`KismetMathLibrary.MakeTransform` (`KismetMathLibrary.MakeVector` (* _index (`self.Distance`))) (struct) (`self.Scale`))))
    (bind _asbp_spear_ejector (cast `/Game/FireAndWater/Blueprints/TempleBoss/BP_SpearEjector` (`ChildActorComponent.ChildActor` _returnvalue)))
    (`KismetArrayLibrary.Array_Add` (`self.Ejectors`) _asbp_spear_ejector)))