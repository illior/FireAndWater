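; BP_TempleSpear is a spear actor for the temple boss content, with launched and takeable states.
; Each tick it draws a green debug sphere at its location while it is unlaunched, takeable and has collision enabled.
; The graph holds only this debug visualization, with no launch or pickup logic, and the construction script is empty.
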(event `self.ReceiveTick`
  (params (DeltaSeconds :type "Float (single-precision)"))
  (`|ExecutionSequence`
    (:`then_0`
      (if (and (not (`self.bLaunched`)) (`self.bTakeable`) (`|EnumInequality` (`PrimitiveComponent.GetCollisionEnabled` (`self.CollisionComponent`)) "NoCollision"))
        (`KismetSystemLibrary.DrawDebugSphere` (`self.K2_GetActorLocation`) 30.0 12 (struct :`G` 1.0 :`A` 1.0))))))

(fn `UserConstructionScript`)