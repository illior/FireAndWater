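; BP_Spear is a projectile in the TempleBoss content that reacts to collision overlaps, ignoring its owner.
; Pawns take damage, and those with a CharacterMovementComponent are launched along the spear's forward vector, after which the spear is destroyed.
; On any other actor, it stops, attaches in place with gravity and collision off, and expires after a short lifespan.
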(event `self.ReceiveBeginPlay`
  (add `PrimitiveComponent.OnComponentBeginOverlap` (`self.Collision`) (delegate `OnComponentBeginOverlap_Event`)))

(event `OnComponentBeginOverlap_Event`
  (params (OverlappedComponent :type "PrimitiveComponent Object Reference") (OtherActor :type "Actor Object Reference") (OtherComp :type "PrimitiveComponent Object Reference") (OtherBodyIndex :type Integer) (bFromSweep :type Boolean) (SweepResult :type "HitResult Structure (by ref)"))
  (bind _returnvalue (`self.GetComponentByClass` OtherActor "/Script/Engine.CharacterMovementComponent"))
  (bind _projectilemovement (`self.ProjectileMovement`))
  (if (!= OtherActor (`self.GetOwner`))
    (if (`GameplayStatics.ObjectIsA` OtherActor "/Script/Engine.Pawn")
      (`GameplayStatics.ApplyDamage` OtherActor 50.0)
      (`/Engine/EditorBlueprintResources/StandardMacros.IsValid` _returnvalue
        (:`Is Valid`
          (`CharacterMovementComponent.AddImpulse` _returnvalue (* (`self.GetActorForwardVector`) 5000.0) true)
          (`self.K2_DestroyActor`)))
      (else
        (`MovementComponent.StopMovementImmediately` _projectilemovement)
        (set `ProjectileMovementComponent.ProjectileGravityScale` 0.0 _projectilemovement)
        (`self.K2_AttachToActor` OtherActor "None" "KeepWorld" "KeepWorld" "KeepWorld")
        (`PrimitiveComponent.SetCollisionEnabled` (`self.Collision`) "NoCollision")
        (`self.SetLifeSpan` 5.0)))))

(fn `UserConstructionScript`)