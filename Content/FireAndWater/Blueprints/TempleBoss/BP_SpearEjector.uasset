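; BP_SpearEjector is a temple boss trap actor that fires a spear when Shot is called, either immediately or after a telegraphed delay.
; With a delay, a looping once-per-frame timer shrinks a red debug sphere at the spawn point over that time, then fires and clears itself.
; Push spawns a non-takeable BP_TempleSpear at the SpearSpawn transform and launches it forward at fixed speed without gravity.
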(event `Shot`
  (if (> (`self.Delay`) 0.0)
    (bind _returnvalue (`KismetSystemLibrary.K2_SetTimerDelegate` (delegate `CustomEvent`) 0.001 true true))
    (set `self.TimerHandle` _returnvalue)
    (`KismetSystemLibrary.DrawDebugSphere` (`SceneComponent.K2_GetComponentLocation` (`self.SpearSpawn`)) (`self.InitialRadius`) 12 (struct :`R` 1.0 :`A` 1.0))
    (set `self.CurrentRadius` (`self.InitialRadius`))
    (else
      (`self.Push`))))

(event `CustomEvent`
  (bind _output_get (set `self.CurrentRadius` (- (`self.CurrentRadius`) (* (/ (`self.InitialRadius`) (`self.Delay`)) (`GameplayStatics.GetWorldDeltaSeconds`)))))
  (if (<= _output_get 0.0)
    (`self.Push`)
    (`KismetSystemLibrary.K2_ClearAndInvalidateTimerHandle` (`self.TimerHandle`))
    (else
      (`KismetSystemLibrary.DrawDebugSphere` (`SceneComponent.K2_GetComponentLocation` (`self.SpearSpawn`)) (`self.CurrentRadius`) 12 (struct :`R` 1.0 :`A` 1.0)))))

(event `Push`
  (bind (_returnvalue_location _returnvalue_rotation) (`KismetMathLibrary.BreakTransform` (`SceneComponent.K2_GetComponentToWorld` (`self.SpearSpawn`))))
  (bind _returnvalue (`|SpawnActorFromClass` "/Game/FireAndWater/Blueprints/TempleBoss/BP_TempleSpear.BP_TempleSpear_C" (`KismetMathLibrary.MakeTransform` _returnvalue_location _returnvalue_rotation) "AlwaysSpawn" "MultiplyWithRoot" self null))
  (set `FAWSpear.bTakeable` false _returnvalue)
  (`FAWSpear.LaunchForward` _returnvalue 2500.0 2500.0 0.0))

(fn `UserConstructionScript`)