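; BP_TakeableSpear is a temple boss spear projectile that, once launched, flies to a target location along a curve-driven arc.
; Tick steps X and Y linearly over the curve's duration, blends Z by curve value, faces the next point and draws debug spheres.
; On overlap, ignoring its owner and other spears, it damages and vanishes on Pawns, or sticks to anything else and expires shortly after.
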(event `self.ReceiveTick`
  (params (DeltaSeconds :type "Float (single-precision)"))
  (bind _position (`self.GetNextPosition` 1))
  (if (and (`self.IsLaunched`) (< (`self.CurrentTime`) (`.MaxTime` (`CurveBase.GetTimeRange` (`self.Trajectory`)))))
    (set `self.CurrentTime` (+ (`self.CurrentTime`) (`GameplayStatics.GetWorldDeltaSeconds`)))
    (`self.K2_SetActorLocationAndRotation` _position (`KismetMathLibrary.SelectRotator` (`KismetMathLibrary.FindLookAtRotation` _position (`self.GetNextPosition` 2)) (`self.K2_GetActorRotation`) (not (`KismetMathLibrary.NearlyEqual_FloatFloat` (`self.CurrentTime`) (`.MaxTime` (`CurveBase.GetTimeRange` (`self.Trajectory`))) (`GameplayStatics.GetWorldDeltaSeconds`)))))
    (`KismetSystemLibrary.DrawDebugSphere` (`self.K2_GetActorLocation`) 10.0 12 (struct :`R` 1.0 :`A` 1.0) 5.0)
    (elif (`self.IsLaunched`)
      _)))

(event `Launch`
  (params (Location :type "Vector Structure") (Trajectory :type "CurveFloat Object Reference"))
  (set `self.IsLaunched` true)
  (set `self.TargetLocation` Location)
  (set `self.Trajectory` Trajectory)
  (set `self.InitialLocation` (`self.K2_GetActorLocation`))
  (set `self.InitialRotation` (`self.K2_GetActorRotation`))
  (set `self.CurrentTime` 0.0))

(event `self.ReceiveBeginPlay`
  (add `PrimitiveComponent.OnComponentBeginOverlap` (`self.Collision`) (delegate `OnComponentBeginOverlap_Event`)))

(event `OnComponentBeginOverlap_Event`
  (params (OverlappedComponent :type "PrimitiveComponent Object Reference") (OtherActor :type "Actor Object Reference") (OtherComp :type "PrimitiveComponent Object Reference") (OtherBodyIndex :type Integer) (bFromSweep :type Boolean) (SweepResult :type "HitResult Structure (by ref)"))
  (bind _projectilemovement (`self.ProjectileMovement`))
  (bind _collision (`self.Collision`))
  (if (and (!= OtherActor (`self.GetOwner`)) (`self.IsLaunched`) (not (`GameplayStatics.ObjectIsA` OtherActor (`GameplayStatics.GetObjectClass` self))))
    (if (`GameplayStatics.ObjectIsA` OtherActor "/Script/Engine.Pawn")
      (`GameplayStatics.ApplyDamage` OtherActor 50.0)
      (set `self.IsLaunched` false)
      (`self.K2_DestroyActor`)
      (else
        (`MovementComponent.StopMovementImmediately` _projectilemovement)
        (set `ProjectileMovementComponent.ProjectileGravityScale` 0.0 _projectilemovement)
        (`self.K2_AttachToActor` OtherActor "None" "KeepWorld" "KeepWorld" "KeepWorld")
        (set `self.IsLaunched` false)
        (`self.SetLifeSpan` 3.0)
        (`/Engine/EditorBlueprintResources/StandardMacros.IsValid` _collision
          (:`Is Valid`
            (`PrimitiveComponent.SetCollisionEnabled` _collision "NoCollision")))))))

(fn `GetNextPosition`
  (params (NewParam :type Integer))
  (returns (Position :type "Vector Structure"))
  (bind (_returnvalue_x _returnvalue_y) (`KismetMathLibrary.BreakVector` (`self.K2_GetActorLocation`)))
  (bind _returnvalue_x_2 (`KismetMathLibrary.BreakVector` (`self.K2_GetActorLocation`)))
  (bind _returnvalue (- NewParam 1))
  (bind (_initiallocation_x _initiallocation_y) (`KismetMathLibrary.BreakVector` (`self.InitialLocation`)))
  (bind (_targetlocation_x _targetlocation_y) (`KismetMathLibrary.BreakVector` (`self.TargetLocation`)))
  (bind _initiallocation_x_2 (`KismetMathLibrary.BreakVector` (`self.InitialLocation`)))
  (bind _targetlocation_x_2 (`KismetMathLibrary.BreakVector` (`self.TargetLocation`)))
  (bind (_targetlocation_x_3 _targetlocation_y_2 _targetlocation_z) (`KismetMathLibrary.BreakVector` (`self.TargetLocation`)))
  (bind (_returnvalue_x_3 _returnvalue_y_2 _returnvalue_z) (`KismetMathLibrary.BreakVector` (+ (`self.InitialLocation`) (* (`KismetMathLibrary.GetForwardVector` (`self.InitialRotation`)) (* (`KismetMathLibrary.Vector_Distance` (`self.TargetLocation`) (`self.InitialLocation`)) (+ (`self.CurrentTime`) (* _returnvalue (`GameplayStatics.GetWorldDeltaSeconds`))))))))
  (return (`KismetMathLibrary.MakeVector` (+ _returnvalue_x_2 (* NewParam (* (/ (* (- _initiallocation_x_2 _targetlocation_x_2) -1.0) (`.MaxTime` (`CurveBase.GetTimeRange` (`self.Trajectory`)))) (`GameplayStatics.GetWorldDeltaSeconds`)))) (+ _returnvalue_y (* NewParam (* (/ (* (- _initiallocation_y _targetlocation_y) -1.0) (`.MaxTime` (`CurveBase.GetTimeRange` (`self.Trajectory`)))) (`GameplayStatics.GetWorldDeltaSeconds`)))) (`KismetMathLibrary.Lerp` _targetlocation_z _returnvalue_z (`CurveFloat.GetFloatValue` (`self.Trajectory`) (+ (`self.CurrentTime`) (* _returnvalue (`GameplayStatics.GetWorldDeltaSeconds`))))))))

(fn `UserConstructionScript`)