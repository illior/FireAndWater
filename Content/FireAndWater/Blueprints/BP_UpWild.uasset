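; Updraft actor that lifts FAWBaseCharacters that overlap it, with all logic running on the server.
; On overlap it adds an upward boost to their vertical velocity, waits two ticks, then switches them to Flying.
; After a short delay, characters still Flying get a much stronger vertical launch.
; Ending the overlap returns them to Falling.
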(event `self.ReceiveActorBeginOverlap`
  (params (OtherActor :type "Actor Object Reference"))
  (`/Engine/EditorBlueprintResources/ActorMacros.Switch Has Authority`
    (:`Authority`
      (bind _asfawbase_character (cast `FAWBaseCharacter` OtherActor))
      (bind (_returnvalue_x _returnvalue_y _returnvalue_z) (`KismetMathLibrary.BreakVector` (`self.GetVelocity` _asfawbase_character)))
      (`Character.LaunchCharacter` _asfawbase_character (`KismetMathLibrary.MakeVector` 0.0 0.0 (+ _returnvalue_z 300.0)) false true)
      (`KismetSystemLibrary.DelayUntilNextTick`)
      (`KismetSystemLibrary.DelayUntilNextTick`)
      (`CharacterMovementComponent.SetMovementMode` (`Character.CharacterMovement` _asfawbase_character) "MOVE_Flying" 0)
      (`KismetSystemLibrary.Delay` 0.75)
      (if (`|EnumEquality` (`CharacterMovementComponent.MovementMode` (`Character.CharacterMovement` _asfawbase_character)) "MOVE_Flying")
        (`Character.LaunchCharacter` _asfawbase_character (0.0 0.0 1500.0) false true)))))

(event `self.ReceiveActorEndOverlap`
  (params (OtherActor :type "Actor Object Reference"))
  (`/Engine/EditorBlueprintResources/ActorMacros.Switch Has Authority`
    (:`Authority`
      (bind _asfawbase_character (cast `FAWBaseCharacter` OtherActor))
      (`CharacterMovementComponent.SetMovementMode` (`Character.CharacterMovement` _asfawbase_character) "MOVE_Falling" 0))))

(fn `UserConstructionScript`)