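; BP_Button is a pressure button that stays pressed while any actor overlaps its collision.
; The authority tracks overlapping actors in a list, firing pressed on the first entry and unpressed when the list empties.
; The construction script binds those dispatchers to events that play or reverse a timeline, easing the mesh's Z position between start and finish heights with a configurable interpolation function.
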(event `self.ButtonCollision.OnComponentBeginOverlap`
  (params (OverlappedComponent :type "PrimitiveComponent Object Reference") (OtherActor :type "Actor Object Reference") (OtherComp :type "PrimitiveComponent Object Reference") (OtherBodyIndex :type Integer) (bFromSweep :type Boolean) (SweepResult :type "HitResult Structure (by ref)"))
  (`/Engine/EditorBlueprintResources/ActorMacros.Switch Has Authority`
    (:`Authority`
      (`KismetArrayLibrary.Array_Add` (`self.ActorsOnButtons`) OtherActor)
      (if (not (`self.IsPressed`))
        (set `self.IsPressed` true)
        (`self.ButtonPressed`)))))

(event `self.ButtonCollision.OnComponentEndOverlap`
  (params (OverlappedComponent :type "PrimitiveComponent Object Reference") (OtherActor :type "Actor Object Reference") (OtherComp :type "PrimitiveComponent Object Reference") (OtherBodyIndex :type Integer))
  (bind _actorsonbuttons (`self.ActorsOnButtons`))
  (`/Engine/EditorBlueprintResources/ActorMacros.Switch Has Authority`
    (:`Authority`
      (`KismetArrayLibrary.Array_RemoveItem` _actorsonbuttons OtherActor)
      (if (== (`KismetArrayLibrary.Array_Length` _actorsonbuttons) 0)
        (set `self.IsPressed` false)
        (`self.ButtonUnpressed`)))))

(event `ButtonPressed_Event`
  (bind _staticmesh (`self.StaticMesh`))
  (bind (_relativelocation_x _relativelocation_y) (`KismetMathLibrary.BreakVector` (`SceneComponent.RelativeLocation` _staticmesh)))
  (bind (_direction _alpha) (`Timeline|ButtonTimeline` :!label _label)
    (:`Update`
      (`SceneComponent.K2_SetRelativeLocation` _staticmesh (`KismetMathLibrary.MakeVector` _relativelocation_x _relativelocation_y (`|EaseFunction` (`self.InterpolateFunction`) _alpha (`self.StartZPostion`) (`self.FinishZPosition`))) false false))))

(event `ButtonUnpressed_Event`
  (goto _label :!via `Reverse`))

(fn `UserConstructionScript`
  (add `self.ButtonPressed` (`|CreateDelegate` :!event `ButtonPressed_Event`))
  (add `self.ButtonUnpressed` (`|CreateDelegate` :!event `ButtonUnpressed_Event`)))