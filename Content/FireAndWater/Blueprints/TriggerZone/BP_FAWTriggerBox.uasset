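; BP_FAWTriggerBox is a trigger zone for Fire and Water that fires when two characters stand inside it at the same time.
; Overlap begin and end events add and remove Characters in a Players array.
; When the array reaches two, it calls the BothPlayersInside dispatcher with that array, then sets collision to NoCollision and clears the array, making the trigger one-shot.
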(event `self.ReceiveActorBeginOverlap`
  (params (OtherActor :type "Actor Object Reference"))
  (bind _ascharacter (cast `Character` OtherActor))
  (`KismetArrayLibrary.Array_Add` (`self.Players`) _ascharacter)
  (if (== (`KismetArrayLibrary.Array_Length` (`self.Players`)) 2)
    (`self.BothPlayersInside` (`self.Players`))
    (`PrimitiveComponent.SetCollisionProfileName` (`self.CollisionComponent`) "NoCollision" true)
    (`KismetArrayLibrary.Array_Clear` (`self.Players`))))

(event `self.ReceiveActorEndOverlap`
  (params (OtherActor :type "Actor Object Reference"))
  (bind _ascharacter (cast `Character` OtherActor))
  (`KismetArrayLibrary.Array_RemoveItem` (`self.Players`) _ascharacter))

(fn `UserConstructionScript`)