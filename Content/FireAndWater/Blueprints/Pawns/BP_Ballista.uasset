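; Possessable, networked ballista pawn that stores stacked spears and fires the last one added along a curve-shaped trajectory.
; On possession it saves and narrows camera view limits; the aim input restores them and repossesses the previous pawn.
; Each tick the controlling player's look rotation turns the replicated meshes via a server event, applied immediately on clients too.
; Animated debug arrows preview the flight path using the same curve, length and height drop.
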(event `MakeShot`
  (bind _arrow (`self.Arrow`))
  (bind _returnvalue (`KismetArrayLibrary.Array_Length` (`self.Spears`)))
  (bind _output (`|GetArrayItem` (`self.Spears`) (- _returnvalue 1)))
  (if (> _returnvalue 0)
    (`self.K2_DetachFromActor` _output "KeepWorld" "KeepWorld" "KeepWorld")
    (`self.K2_SetActorTransform` _output (`SceneComponent.K2_GetComponentToWorld` (`self.Arrow`)) false false)
    (`self.SetOwner` _output self)
    (`FAWSpear.LaunchAlongTrajectory` _output (`KismetMathLibrary.MakeVector` (.x (+ (`SceneComponent.K2_GetComponentLocation` _arrow) (* (`SceneComponent.GetForwardVector` _arrow) (`self.ProjectileTrajectoryLenght`)))) (.y (+ (`SceneComponent.K2_GetComponentLocation` _arrow) (* (`SceneComponent.GetForwardVector` _arrow) (`self.ProjectileTrajectoryLenght`)))) (- (.z (+ (`SceneComponent.K2_GetComponentLocation` _arrow) (* (`SceneComponent.GetForwardVector` _arrow) (`self.ProjectileTrajectoryLenght`)))) (`self.ProjectileHeight`))) (`self.ProjectileTrajectory`))
    (set `FAWSpear.bTakeable` false _output)
    (`KismetArrayLibrary.Array_RemoveItem` (`self.Spears`) _output)))

(event `ServerFire`
  (`self.MakeShot`))

(event `EnhancedInput|/Game/FireAndWater/Players/Input/IA_Fire`
  (params (ActionValue :type Boolean) (ElapsedSeconds :type "Float (double-precision)") (TriggeredSeconds :type "Float (double-precision)") (InputAction :type "InputAction Object Reference" :default "/Game/FireAndWater/Players/Input/IA_Fire.IA_Fire"))
  (:`Started`
    (`self.ServerFire`)))

(event `AddSpear`
  (params (InSpear :type "FAWSpear Object Reference"))
  (bind (_returnvalue_x _returnvalue_y _returnvalue_z) (`KismetMathLibrary.BreakVector` (`SceneComponent.K2_GetComponentLocation` (`self.SpearsHolder`))))
  (`self.K2_AttachToComponent` InSpear (`self.SpearsHolder`) "None" "KeepWorld" "KeepWorld" "KeepWorld" true)
  (`self.K2_SetActorLocationAndRotation` InSpear (`KismetMathLibrary.MakeVector` _returnvalue_x _returnvalue_y (+ _returnvalue_z (* 20.0 (`KismetArrayLibrary.Array_Length` (`self.Spears`))))) (`SceneComponent.K2_GetComponentRotation` (`self.SpearsHolder`)) false false)
  (`KismetArrayLibrary.Array_Add` (`self.Spears`) InSpear))

(event `EnhancedInput|/Game/FireAndWater/Players/Input/IA_Look`
  (params (ActionValue :type "Vector2D Structure") (ElapsedSeconds :type "Float (double-precision)") (TriggeredSeconds :type "Float (double-precision)") (InputAction :type "InputAction Object Reference" :default "/Game/FireAndWater/Players/Input/IA_Look.IA_Look"))
  (bind (_x _y) (`KismetMathLibrary.BreakVector2D` ActionValue))
  (:`Triggered`
    (`self.AddControllerYawInput` _x)
    (`self.AddControllerPitchInput` _y)))

(event `EnhancedInput|/Game/FireAndWater/Players/Input/IA_Aim`
  (params (ActionValue :type Boolean) (ElapsedSeconds :type "Float (double-precision)") (TriggeredSeconds :type "Float (double-precision)") (InputAction :type "InputAction Object Reference" :default "/Game/FireAndWater/Players/Input/IA_Aim.IA_Aim"))
  (:`Started`
    (`self.ServerReturnToPawn`)))

(event `ServerReturnToPawn`
  (`self.ReturnToPawn`))

(event `self.ReceiveBeginPlay`
  (add `self.ReceiveControllerChangedDelegate` (`|CreateDelegate` :!event `ReceiveControllerChangedDelegate_Event`)))

(event `/Game/FireAndWater/Blueprints/Pawns/BPI_TempControlledPawn.SetPawnToReturn`
  (params (InPawn :type "Pawn Object Reference"))
  (set `self.PawnToReturn` InPawn))

(event `/Game/FireAndWater/Blueprints/Pawns/BPI_TempControlledPawn.ReturnToPawn`
  (bind _staticmesh (`self.StaticMesh`))
  (bind _staticmesh1 (`self.StaticMesh1`))
  (bind (_relativerotation_roll _relativerotation_pitch) (`KismetMathLibrary.BreakRotator` (`SceneComponent.RelativeRotation` _staticmesh1)))
  (bind (_relativerotation_roll_2 _relativerotation_pitch_2) (`KismetMathLibrary.BreakRotator` (`SceneComponent.RelativeRotation` _staticmesh)))
  (`self.ResetCameraSettings`)
  (`Controller.Possess` (`self.GetController`) (`self.PawnToReturn`))
  (`SceneComponent.K2_SetRelativeRotation` _staticmesh (`KismetMathLibrary.MakeRotator` _relativerotation_roll_2 _relativerotation_pitch_2) false false)
  (`SceneComponent.K2_SetRelativeRotation` _staticmesh1 (`KismetMathLibrary.MakeRotator` _relativerotation_roll _relativerotation_pitch) false false))

(event `ResetCameraSettings`
  (bind (_oldcamerayaw_x _oldcamerayaw_y) (`KismetMathLibrary.BreakVector2D` (`self.OldCameraYaw`)))
  (bind (_oldcamerapitch_x _oldcamerapitch_y) (`KismetMathLibrary.BreakVector2D` (`self.OldCameraPitch`)))
  (bind _asplayer_controller (cast `PlayerController` (`self.GetController`)))
  (bind _playercameramanager (`PlayerController.PlayerCameraManager` _asplayer_controller))
  (set `PlayerCameraManager.ViewPitchMin` _oldcamerapitch_x _playercameramanager)
  (set `PlayerCameraManager.ViewPitchMax` _oldcamerapitch_y _playercameramanager)
  (set `PlayerCameraManager.ViewYawMin` _oldcamerayaw_x _playercameramanager)
  (set `PlayerCameraManager.ViewYawMax` _oldcamerayaw_y _playercameramanager))

(event `ReceiveControllerChangedDelegate_Event` :!signature `self.ReceiveControllerChangedDelegate`
  (params (Pawn :type "Pawn Object Reference") (OldController :type "Controller Object Reference") (NewController :type "Controller Object Reference"))
  (bind (_returnvalue_roll _returnvalue_pitch _returnvalue_yaw) (`KismetMathLibrary.BreakRotator` (`self.K2_GetActorRotation`)))
  (`/Engine/EditorBlueprintResources/StandardMacros.IsValid` NewController
    (:`Is Valid`
      (bind _asplayer_controller (cast `PlayerController` NewController))
      (bind _playercameramanager (`PlayerController.PlayerCameraManager` _asplayer_controller))
      (set `self.OldCameraPitch` (`KismetMathLibrary.MakeVector2D` (`PlayerCameraManager.ViewPitchMin` _playercameramanager) (`PlayerCameraManager.ViewPitchMax` _playercameramanager)))
      (set `self.OldCameraYaw` (`KismetMathLibrary.MakeVector2D` (`PlayerCameraManager.ViewYawMin` _playercameramanager) (`PlayerCameraManager.ViewYawMax` _playercameramanager)))
      (set `PlayerCameraManager.ViewPitchMax` 30.0 _playercameramanager)
      (set `PlayerCameraManager.ViewPitchMin` -10.0 _playercameramanager)
      (set `PlayerCameraManager.ViewYawMin` (- _returnvalue_yaw 40.0) _playercameramanager)
      (set `PlayerCameraManager.ViewYawMax` (+ _returnvalue_yaw 40.0) _playercameramanager))))

(event `ServerSetRotation`
  (params (InControlRotation :type "Rotator Structure"))
  (bind (_returnvalue_roll _returnvalue_pitch _returnvalue_yaw) (`KismetMathLibrary.BreakRotator` (`self.K2_GetActorRotation`)))
  (bind _staticmesh (`self.StaticMesh`))
  (bind _staticmesh1 (`self.StaticMesh1`))
  (bind (_relativerotation_roll _relativerotation_pitch) (`KismetMathLibrary.BreakRotator` (`SceneComponent.RelativeRotation` _staticmesh)))
  (bind (_relativerotation_roll_2 _relativerotation_pitch_2) (`KismetMathLibrary.BreakRotator` (`SceneComponent.RelativeRotation` _staticmesh1)))
  (`SceneComponent.K2_SetRelativeRotation` _staticmesh (`KismetMathLibrary.MakeRotator` _relativerotation_roll _relativerotation_pitch (- (.yaw InControlRotation) _returnvalue_yaw)) false false)
  (`SceneComponent.K2_SetRelativeRotation` _staticmesh1 (`KismetMathLibrary.MakeRotator` _relativerotation_roll_2 _relativerotation_pitch_2 (.pitch InControlRotation)) false false))

(event `self.ReceiveTick`
  (params (DeltaSeconds :type "Float (single-precision)"))
  (bind _returnvalue (`self.GetControlRotation`))
  (bind (_returnvalue_roll _returnvalue_pitch _returnvalue_yaw) (`KismetMathLibrary.BreakRotator` (`self.K2_GetActorRotation`)))
  (bind _staticmesh1 (`self.StaticMesh1`))
  (bind _staticmesh (`self.StaticMesh`))
  (bind (_relativerotation_roll _relativerotation_pitch) (`KismetMathLibrary.BreakRotator` (`SceneComponent.RelativeRotation` _staticmesh)))
  (bind (_relativerotation_roll_2 _relativerotation_pitch_2) (`KismetMathLibrary.BreakRotator` (`SceneComponent.RelativeRotation` _staticmesh1)))
  (if (and (`KismetSystemLibrary.IsValid` (`self.GetController`)) (`self.IsLocallyControlled`))
    (`/Engine/EditorBlueprintResources/ActorMacros.Switch Has Authority`
      (:`Authority`
        _)
      (:`Remote`
        (`SceneComponent.K2_SetRelativeRotation` _staticmesh (`KismetMathLibrary.MakeRotator` _relativerotation_roll _relativerotation_pitch (- (.yaw _returnvalue) _returnvalue_yaw)) false false)
        (`SceneComponent.K2_SetRelativeRotation` _staticmesh1 (`KismetMathLibrary.MakeRotator` _relativerotation_roll_2 _relativerotation_pitch_2 (.pitch _returnvalue)) false false)))
    (`self.ServerSetRotation` (`self.GetControlRotation`))
    (`self.DrawProjectileTrajectory`)))

(event `DrawProjectileTrajectory`
  (bind _arrow (`self.Arrow`))
  (bind _returnvalue (`SceneComponent.K2_GetComponentLocation` _arrow))
  (bind _returnvalue_2 (`SceneComponent.GetForwardVector` _arrow))
  (bind _returnvalue_3 (+ (* (`self.ArrowSpeed`) (`GameplayStatics.GetWorldDeltaSeconds`)) (`self.ArrowPosition`)))
  (for _index (range (`self.ArrowsCount`))
    (bind _returnvalue_4 (+ (`self.ArrowPosition`) (* _index (/ (`self.ProjectileTrajectoryLenght`) (`self.ArrowsCount`)))))
    (bind (_returnvalue_x _returnvalue_y _returnvalue_z) (`KismetMathLibrary.BreakVector` (+ (* _returnvalue_2 _returnvalue_4) _returnvalue)))
    (bind _returnvalue_5 (+ _returnvalue_4 50.0))
    (bind (_returnvalue_x_2 _returnvalue_y_2 _returnvalue_z_2) (`KismetMathLibrary.BreakVector` (+ (* _returnvalue_2 _returnvalue_5) _returnvalue)))
    (`KismetSystemLibrary.DrawDebugArrow` (`KismetMathLibrary.MakeVector` _returnvalue_x _returnvalue_y (- _returnvalue_z (* (- 1.0 (`CurveFloat.GetFloatValue` (`self.ProjectileTrajectory`) (/ _returnvalue_4 (`self.ProjectileTrajectoryLenght`)))) (`self.ProjectileHeight`)))) (`KismetMathLibrary.MakeVector` _returnvalue_x_2 _returnvalue_y_2 (- _returnvalue_z_2 (* (- 1.0 (`CurveFloat.GetFloatValue` (`self.ProjectileTrajectory`) (/ _returnvalue_5 (`self.ProjectileTrajectoryLenght`)))) (`self.ProjectileHeight`)))) 50.0 (struct :`R` 1.0 :`A` 1.0) 0.0 7.0)
    (set `self.ArrowPosition` (`KismetMathLibrary.SelectFloat` 0.0 _returnvalue_3 (> _returnvalue_3 (/ (`self.ProjectileTrajectoryLenght`) (`self.ArrowsCount`)))))))

(fn `UserConstructionScript`
  (`ActorComponent.SetIsReplicated` (`self.StaticMesh`) true)
  (`ActorComponent.SetIsReplicated` (`self.StaticMesh1`) true))