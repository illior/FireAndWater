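; BP_Lever is an interactable lever that switches an Active state and broadcasts it through an OnMoved dispatcher.
; BeginPlay poses the handle to match Active and binds interaction events: a press toggles the lever, while in ShouldHold mode completing a hold activates it and cancelling deactivates it.
; A looping timer pitches the handle toward either limit using delta time, scaling speed by HoldTime in hold mode.
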(event `self.ReceiveBeginPlay`
  (`SceneComponent.K2_SetRelativeRotation` (`self.Handle`) (`KismetMathLibrary.MakeRotator` 0.0 (`KismetMathLibrary.SelectFloat` -30.0 30.0 (`self.bActive`))) false false)
  (add `self.OnStartInteract` (`|CreateDelegate` :!event `OnStartInteract_Event`))
  (add `self.OnCompleteHold` (`|CreateDelegate` :!event `OnCompleteHold_Event`))
  (add `self.OnCancelHold` (`|CreateDelegate` :!event `OnCancelHold_Event`)))

(event `OnCancelHold_Event` :!signature `self.OnCancelHold`
  (params (ActivatedActor :type "FAWInteractableActor Object Reference") (ActivatedBy :type "Pawn Object Reference"))
  (`self.StartMoveHandle` 30.0)
  (bind _output_get (set `self.bActive` false))
  (`self.OnMoved` _output_get))

(event `OnCompleteHold_Event` :!signature `self.OnCompleteHold`
  (params (ActivatedActor :type "FAWInteractableActor Object Reference") (ActivatedBy :type "Pawn Object Reference"))
  (`self.StartMoveHandle` -30.0)
  (bind _output_get (set `self.bActive` true))
  (`self.OnMoved` _output_get))

(event `OnStartInteract_Event` :!signature `self.OnStartInteract`
  (params (ActivatedActor :type "FAWInteractableActor Object Reference") (ActivatedBy :type "Pawn Object Reference"))
  (if (not (`self.ShouldHold`))
    (if (`self.bActive`)
      (`self.StartMoveHandle` 30.0)
      (bind _output_get (set `self.bActive` false))
      (`self.OnMoved` _output_get)
      (else
        (`self.StartMoveHandle` -30.0)
        (bind _output_get_2 (set `self.bActive` true))
        (`self.OnMoved` _output_get_2)))))

(event `StartMoveHandle`
  (params (Angle :type "Float (double-precision)"))
  (set `self.TargetAngle` Angle)
  (bind _returnvalue (`KismetSystemLibrary.K2_SetTimerDelegate` (delegate `MoveHandle`) 0.005 true true))
  (set `self.TimerHandle` _returnvalue))

(event `MoveHandle`
  (bind _handle (`self.Handle`))
  (bind (_relativerotation_roll _relativerotation_pitch _relativerotation_yaw) (`KismetMathLibrary.BreakRotator` (`SceneComponent.RelativeRotation` _handle)))
  (bind _returnvalue (+ _relativerotation_pitch (* (* (* 60.0 (`KismetMathLibrary.SignOfFloat` (`self.TargetAngle`))) (select `bool` (`self.ShouldHold`) :`false` 1.0 :`true` (/ 1.0 (`self.HoldTime`)) :!type "Float (single-precision)")) (`GameplayStatics.GetWorldDeltaSeconds`))))
  (`SceneComponent.K2_SetRelativeRotation` _handle (`KismetMathLibrary.MakeRotator` _relativerotation_roll _returnvalue _relativerotation_yaw) false false)
  (if (> (`KismetMathLibrary.Abs` _returnvalue) 30.0)
    (`KismetSystemLibrary.K2_ClearAndInvalidateTimerHandle` (`self.TimerHandle`))))

(fn `UserConstructionScript`)