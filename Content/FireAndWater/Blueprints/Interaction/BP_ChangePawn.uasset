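; BP_ChangePawn is a hold-to-interact object that moves the activating player's controller into another pawn.
; On hold completion it spawns the configured pawn class at SpawnLocation on first use, reuses it while valid, and possesses it.
; It passes the original pawn to the new one as the pawn to return to.
; When the spawned pawn loses its controller, a multicast call re-enables the interaction.
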(event `OnCompleteHold_Event`
  (params (ActivatedActor :type "FAWInteractableActor Object Reference") (ActivatedBy :type "Pawn Object Reference"))
  (`self.CreateAndPossessPawn` ActivatedBy))

(event `Changed`
  (params (Pawn :type "Pawn Object Reference") (OldController :type "Controller Object Reference") (NewController :type "Controller Object Reference"))
  (`/Engine/EditorBlueprintResources/StandardMacros.IsValid` NewController
    (:`Is Not Valid`
      (`self.Multicast_SetEnabled` true))))

(fn `CreateAndPossessPawn`
  (params (Instigator :type "Pawn Object Reference"))
  (locals (Controller :type "Controller Object Reference"))
  (set `local.Controller` (`Pawn.GetController` Instigator))
  (`/Engine/EditorBlueprintResources/StandardMacros.IsValid` (`self.NewPawnRef`)
    (:`Is Valid`
      _)
    (:`Is Not Valid`
      (bind _returnvalue (`|SpawnActorFromClass` (`self.NewPawnClass`) (`SceneComponent.K2_GetComponentToWorld` (`self.SpawnLocation`)) "Undefined" "MultiplyWithRoot" null null))
      (bind _output_get (set `self.NewPawnRef` _returnvalue))
      (add `Pawn.ReceiveControllerChangedDelegate` _output_get (`|CreateDelegate` :!event `Changed`))))
  (message `/Game/FireAndWater/Blueprints/Pawns/BPI_TempControlledPawn.SetPawnToReturn` (`self.NewPawnRef`) (`local.Instigator`))
  (`Controller.Possess` (`local.Controller`) (`self.NewPawnRef`)))

(fn `UserConstructionScript`
  (add `self.OnCompleteHold` (`|CreateDelegate` :!event `OnCompleteHold_Event`)))