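; BP_GameMode picks a different default pawn class per player for a Fire and Water game.
; GetDefaultPawnClassForController records the first controller it sees in the Players array and gives it BP_WaterCharacter.
; Every other controller receives BP_FireCharacter, while the first keeps water on later calls.
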(fn `GetDefaultPawnClassForController`
  (params (InController :type "Controller Object Reference"))
  (returns (ReturnValue :type "Object Class Reference"))
  (if (== (`KismetArrayLibrary.Array_Length` (`self.Players`)) 0)
    (`KismetArrayLibrary.Array_Add` (`self.Players`) (`local.InController`))
    (elif (== (`|GetArrayItem` (`self.Players`)) (`local.InController`))
      _
      (else
        (return "/Game/FireAndWater/Players/BP_FireCharacter.BP_FireCharacter_C"))))
  (return "/Game/FireAndWater/Players/BP_WaterCharacter.BP_WaterCharacter_C"))

(fn `UserConstructionScript`)