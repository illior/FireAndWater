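; BP_TestInteract is a test actor for the interaction system that reports its interaction events through debug prints.
; Start, stop, hold-complete and owner-change events each print a message.
; EventOnServer prints, turns on static mesh collision through EnableCollision, then calls MulticastSetEnabled with false.
; Overlap, Enable and Disable events are empty, and several leftover debug chains are never run.
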(event `EnableCollision`
  (params (NewValue :type Boolean))
  (if NewValue
    (`PrimitiveComponent.SetCollisionEnabled` (`self.StaticMesh`) "QueryAndPhysics")
    (else
      (`PrimitiveComponent.SetCollisionEnabled` (`self.StaticMesh`) "NoCollision"))))

(event `self.ReceiveComplete`
  (`KismetSystemLibrary.PrintString` "CompleteHold"))

(event `self.ReceiveStartInteract`
  (`KismetSystemLibrary.PrintString` "Start"))

(event `self.ReceiveStopInteract`
  (`KismetSystemLibrary.PrintString` "Stop"))

(event `self.OwnerChangedZZZ`
  (`KismetSystemLibrary.PrintString` "ZZZ" true true (struct :`A` 1.0) 5.0))

(event `self.ReceiveActorBeginOverlap`
  (params (OtherActor :type "Actor Object Reference")))

(event `EventOnServer`
  (`KismetSystemLibrary.PrintString` "DoSMTOnServer" true true (struct :`A` 1.0))
  (`self.EnableCollision` true)
  (`self.Multicast_SetEnabled` false))

(event `self.ReceiveDisable`)

(event `self.ReceiveEnable`)

(fn `UserConstructionScript`)